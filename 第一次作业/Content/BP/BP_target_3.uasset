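; BP_target_3 is a damageable target with a plane mesh that tilts on a timeline.
; AnyDamage tests TargetHealthinfo before subtracting, so the Box component is destroyed only by a hit that arrives with health already at or below zero.
; A separate rotation event, not called within this Blueprint, plays Light01Cue and runs Timeline_1 to lerp SMTargetPlane's relative rotation.
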(event `self.ReceiveAnyDamage`
  (params (Damage :type "Float (single-precision)") (DamageType :type "DamageType Object Reference") (InstigatedBy :type "Controller Object Reference") (DamageCauser :type "Actor Object Reference"))
  (bind _target_healthinfo (`self.target_healthinfo`))
  (`/Engine/EditorBlueprintResources/StandardMacros.CompareFloat` _target_healthinfo
    (:`>`
      (set `self.target_healthinfo` (- _target_healthinfo Damage)))
    (:`==`
      (`ActorComponent.K2_DestroyComponent` (`self.Box`) :!label _label))
    (:`<`
      (goto _label))))

(event `Event rotation`
  (`AudioComponent.Play` (`self.Light01_Cue`) 0.0)
  (bind (_direction _target_up_value) (`Timeline|Timeline_1` :!via `PlayFromStart`) ; 立起被击倒，反向播放
    (:`Update`
      (`SceneComponent.K2_SetRelativeRotation` (`self.SM_target_plane`) (`KismetMathLibrary.RLerp` (struct) (struct :`Yaw` 30.0) _target_up_value) false false))))

(fn `UserConstructionScript`)