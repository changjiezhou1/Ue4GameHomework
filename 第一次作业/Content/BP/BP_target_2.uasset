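; BP_target_2 is a damageable target actor that awards score when destroyed.
; On AnyDamage it subtracts damage from TargetHealthinfo while that value is above zero.
; The check runs before subtraction, so a hit arriving at zero or less health destroys the actor and prints a message.
; It then adds three points to ScoreTarget on the myscore game instance and prints the total.
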(event `self.ReceiveAnyDamage`
  (params (Damage :type "Float (single-precision)") (DamageType :type "DamageType Object Reference") (InstigatedBy :type "Controller Object Reference") (DamageCauser :type "Actor Object Reference"))
  (bind _target_healthinfo (`self.target_healthinfo`))
  (`/Engine/EditorBlueprintResources/StandardMacros.CompareFloat` _target_healthinfo
    (:`>`
      (set `self.target_healthinfo` (- _target_healthinfo Damage)))
    (:`==`
      (`self.K2_DestroyActor` :!label _label)
      (`KismetSystemLibrary.PrintString` "thsi actor is destoryed.")
      (bind _asmyscore (cast `/Game/BP/myscore` (`GameplayStatics.GetGameInstance`)))
      (bind _output_get (set `/Game/BP/myscore.score_target` (+ (`/Game/BP/myscore.score_target` _asmyscore) 3) _asmyscore))
      (`KismetSystemLibrary.PrintString` (`KismetStringLibrary.Conv_IntToString` _output_get)))
    (:`<`
      (goto _label))))

(fn `UserConstructionScript`)