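; Shootable target that stands up on an event and falls over when its health is depleted, awarding score.
; AnyDamage checks health before subtracting, so the knockdown fires on a hit received when health is already zero or below.
; Knockdown destroys the Box, adds two points to the myscore GameInstance and sets Istargetdown.
; The Target_up timeline rotates the plane mesh, forward to rise and reversed to fall, with a sound cue for each.
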(event `self.ReceiveAnyDamage`
  (params (Damage :type "Float (single-precision)") (DamageType :type "DamageType Object Reference") (InstigatedBy :type "Controller Object Reference") (DamageCauser :type "Actor Object Reference"))
  (bind _target_healthinfo (`self.target_healthinfo`))
  (`/Engine/EditorBlueprintResources/StandardMacros.CompareFloat` _target_healthinfo
    (:`>`
      (set `self.target_healthinfo` (- _target_healthinfo Damage)))
    (:`==`
      (`ActorComponent.K2_DestroyComponent` (`self.Box`) :!label _label)
      (`KismetSystemLibrary.PrintString` "box destroyed!")
      (bind _asmyscore (cast `/Game/BP/myscore` (`GameplayStatics.GetGameInstance`)))
      (bind _output_get (set `/Game/BP/myscore.score_target` (+ (`/Game/BP/myscore.score_target` _asmyscore) 2) _asmyscore))
      (`KismetSystemLibrary.PrintString` (`KismetStringLibrary.Conv_IntToString` _output_get))
      (`AudioComponent.Play` (`self.Light02_Cue`) 0.0)
      (set `self.istargetdown` true)
      (bind (_direction _target_up_value) (`Timeline|target_up` :!via `ReverseFromEnd` :!label _label_2) ; 立起被击倒，反向播放
        (:`Update`
          (`SceneComponent.K2_SetRelativeRotation` (`self.SM_target_plane`) (`KismetMathLibrary.RLerp` (struct) (struct :`Pitch` 90.0) _target_up_value) false false))))
    (:`<`
      (goto _label))))

(event `target_up_event`
  ;[1 1 1] 初始立起音效
  (`AudioComponent.Play` (`self.Light01_Cue`) 0.0)
  (goto _label_2 :!via `PlayFromStart`))

(fn `UserConstructionScript`)