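; BP_target_2_Child is a child target Blueprint that slides back and forth along the world X axis.
; Each Tick, after calling the parent, it steps forward by a fixed offset while one counter fills, then steps back while a second counter fills, then resets both.
; Movement is a per-frame step without sweep and ignores DeltaSeconds, so its speed depends on frame rate.
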(event `self.ReceiveTick`
  (params (DeltaSeconds :type "Float (single-precision)"))
  (bind _returnvalue (`self.K2_GetActorLocation`))
  (`parent.ReceiveTick` DeltaSeconds)
  (if (>= (`self.add`) 100)
    (if (>= (`self.count`) 100)
      (set `self.add` 0)
      (set `self.count` 0)
      (else
        (`self.K2_SetActorLocation` (- _returnvalue (10.0 0.0 0.0)))
        (set `self.count` (+ (`self.count`) 1))))
    (else
      (`self.K2_SetActorLocation` (+ _returnvalue (10.0 0.0 0.0)))
      (set `self.add` (+ (`self.add`) 1)))))

(fn `UserConstructionScript`
  (`parent.UserConstructionScript`))