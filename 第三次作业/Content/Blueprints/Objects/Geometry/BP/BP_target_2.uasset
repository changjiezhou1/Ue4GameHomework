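; BP_target_2 is a damageable target that awards score when destroyed.
; AnyDamage subtracts damage from TargetHealthinfo until it would reach zero or below, then adds three to PlayerScore on ThirdPersonGameMode and destroys the actor.
; The Destroyed event adds one more point, so a kill by damage totals four.
; Debug strings print on every hit and on destruction by damage.
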(event `self.ReceiveAnyDamage`
  (params (Damage :type "Float (single-precision)") (DamageType :type "DamageType Object Reference") (InstigatedBy :type "Controller Object Reference") (DamageCauser :type "Actor Object Reference"))
  (bind _returnvalue (- (`self.target_healthinfo`) Damage))
  (`KismetSystemLibrary.PrintString` "llll")
  (`/Engine/EditorBlueprintResources/StandardMacros.CompareFloat` _returnvalue
    (:`>`
      (set `self.target_healthinfo` _returnvalue))
    (:`==`
      (`KismetSystemLibrary.PrintString` "box destroyed!" :!label _label)
      (bind _asthird_person_game_mode (cast `/Game/ThirdPersonBP/Blueprints/ThirdPersonGameMode` (`GameplayStatics.GetGameMode`)))
      (set `/Game/ThirdPersonBP/Blueprints/ThirdPersonGameMode.PlayerScore` (+ (`/Game/ThirdPersonBP/Blueprints/ThirdPersonGameMode.PlayerScore` _asthird_person_game_mode) 3) _asthird_person_game_mode)
      (`self.K2_DestroyActor` self))
    (:`<`
      (goto _label))))

(event `self.ReceiveDestroyed`
  (bind _asthird_person_game_mode (cast `/Game/ThirdPersonBP/Blueprints/ThirdPersonGameMode` (`GameplayStatics.GetGameMode`)))
  (set `/Game/ThirdPersonBP/Blueprints/ThirdPersonGameMode.PlayerScore` (+ (`/Game/ThirdPersonBP/Blueprints/ThirdPersonGameMode.PlayerScore` _asthird_person_game_mode) 1) _asthird_person_game_mode))

(fn `UserConstructionScript`)