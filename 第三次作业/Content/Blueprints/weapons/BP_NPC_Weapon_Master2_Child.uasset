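; NPC weapon Blueprint, apparently a child of BP_NPC_Weapon_Master2, that defines how the gun fires.
; Its NPC_Fire event spawns a scaled-down BP_NPC_Bullet_Master at the Shootpoint component's world location, oriented by Currentmuzzlerot.
; The construction script only calls the parent, BeginPlay, Tick and overlap are disabled stubs, and leftover muzzle socket and MuzzleRot nodes are unused.
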(event `NPC_Fire`
  ;[1 1 1] 枪械开火逻辑
  (`|SpawnActorFromClass` "/Game/Blueprints/weapons/Projectiles/BP_NPC_Bullet_Master.BP_NPC_Bullet_Master_C" (`KismetMathLibrary.MakeTransform` (`SceneComponent.K2_GetComponentLocation` (`self.shootpoint`)) (`self.Currentmuzzlerot`) (0.3 0.3 0.3)) "Undefined" "OverrideRootScale" null null))

(fn `UserConstructionScript`
  (`parent.UserConstructionScript`))