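; Grenade weapon actor that explodes on a fixed fuse, wiping out nearby test cubes and targets.
; BeginPlay starts a one-shot three-second timer that calls Detonate.
; Detonate spawns an Explosion at the grenade's transform, destroys actors of hard-coded cube and target classes overlapping its Sphere, then destroys itself.
; There is no damage system or impact trigger; each class gets its own overlap query.
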(event `Detonate`
  (`|SpawnActorFromClass` "/Game/Blueprints/weapons/Explosion.Explosion_C" (`self.GetTransform`) "Undefined" "OverrideRootScale" null null)
  (`self.K2_DestroyActor` (`PrimitiveComponent.GetOverlappingActors` (`self.Sphere`) "/Game/Blueprints/Objects/testcube.testcube_C"))
  (`self.K2_DestroyActor` (`PrimitiveComponent.GetOverlappingActors` (`self.Sphere`) "/Game/UI/BP/BP_target.BP_target_C"))
  (`self.K2_DestroyActor` (`PrimitiveComponent.GetOverlappingActors` (`self.Sphere`) "/Game/Blueprints/Objects/Geometry/BP/BP_target_2.BP_target_2_C"))
  (`self.K2_DestroyActor` (`PrimitiveComponent.GetOverlappingActors` (`self.Sphere`) "/Game/Blueprints/Objects/Geometry/BP/BP_target_2_Move.BP_target_2_Move_C"))
  (`self.K2_DestroyActor` (`PrimitiveComponent.GetOverlappingActors` (`self.Sphere`) "/Game/Blueprints/Objects/Geometry/BP/BP_target_2_Move_2.BP_target_2_Move_2_C"))
  (`self.K2_DestroyActor`))

(event `self.ReceiveBeginPlay`
  (`KismetSystemLibrary.K2_SetTimerDelegate` (delegate `Detonate`) 3.0))

(fn `UserConstructionScript`)